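; BP_Beam is a projectile actor that damages what it hits and bursts on impact.
; An event sets the initial speed on its ProjectileMovement component, and construction records the spawn location.
; On a hit, it spawns a burst system aligned to the surface normal and destroys itself.
; It then sends the hit actor a GetHitMessage carrying damage and the original spawn location.
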(event Custom|Set%20Projectile%20Speed
  (params (Initial%20Speed :type Float%20%28double-precision%29))
  (Variables|/Script/Engine.ProjectileMovementComponent|SetInitialSpeed (Variables|Default|GetProjectileMovement) Initial%20Speed))

(event Collision|EventHit
  (params (MyComp :type Primitive%20Component%20Object%20Reference) (Other :type Actor%20Object%20Reference) (OtherComp :type Primitive%20Component%20Object%20Reference) (bSelfMoved :type Boolean) (HitLocation :type Vector :default "0, 0, 0") (HitNormal :type Vector :default "0, 0, 0") (NormalImpulse :type Vector :default "0, 0, 0") (Hit :type Hit%20Result%20Structure%20%28by%20ref%29))
  (CallFunction|HandleHit Other Hit))

(fn ConstructionScript
  (Variables|Default|SetSpawn%20Location (Transformation|GetActorLocation)))

(fn HandleHit
  (params (Other :type Object%20Object%20Reference) (Hit :type Hit%20Result%20Structure%20%28by%20ref%29))
  (bind (_bblockinghit _binitialoverlap _time _distance _location _impactpoint _normal) (Collision|BreakHitResult Hit))
  (Niagara|SpawnSystematLocation (Variables|Settings|GetBurst%20System) _impactpoint (Math|Rotator|MakeRotfromX _normal))
  (Actor|DestroyActor)
  (Class|BPIDamageable|GetHit(Message) Other (Variables|Settings|GetDamage) (Variables|Default|GetSpawn%20Location)))