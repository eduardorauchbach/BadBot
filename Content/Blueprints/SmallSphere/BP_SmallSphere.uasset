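; BP_SmallSphere is a short-lived, drifting collectible sphere that scores a point when a pawn touches it.
; Each tick it moves along its forward vector while spinning by a random rotation set at BeginPlay, so its path curves.
; Pawn overlap increments the BP_Game score, plays a teleport sound and winks it out.
; Timelines scale the mesh in on spawn and out on pickup or lifetime expiry, then destroy the actor.
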(event Custom|Wink%20Out
  ;[0.15 0 0.000862 0.5] Wink Out Timeline
  (if (not (Variables|Default|GetIs%20Winking))
    (Variables|Default|SetIs%20Winking true)
    (bind _scale (Timeline|T%20Wink%20Out Play)
      (:Update
        (CallFunction|UpdateScale _scale))
      (:Finished
        (Actor|DestroyActor)))))

(event Custom|Wink%20In
  (bind _scale (Timeline|T%20Wink%20In Play)
    (:Update
      (Transformation|SetWorldScale3D (Variables|Default|GetSphere%20Mesh) _scale))))

(event Custom|On%20Sphere%20Overlap
  (params (OverlappedComponent :type Primitive%20Component%20Object%20Reference) (OtherActor :type Actor%20Object%20Reference) (OtherComp :type Primitive%20Component%20Object%20Reference) (OtherBodyIndex :type Integer) (bFromSweep :type Boolean) (SweepResult :type Hit%20Result%20Structure%20%28by%20ref%29))
  ;[0.15 0.09377 0 0.5] Sphere Overlap
  (if (Class|GameplayStatics|ObjectIsA OtherActor "/Script/Engine.Pawn")
    (bind _asbp_game (Utilities|Casting|CastToBP_Game (Game|GetGameMode)))
    (Default|IncrementScore _asbp_game)
    (Audio|PlaySoundatLocation "/Engine/VREditor/Sounds/VR_teleport.VR_teleport" (Transformation|GetActorLocation OtherActor) "0, 0, 0" 1.0 1.0 0.0 0 0 0 0)
    (CallFunction|WinkOut)))

(event EventBeginPlay
  (CallFunction|Winkin)
  (CallFunction|InitializeDeltaRotation)
  ;[0.15 0 0.000862 0.5] Wink Out Timeline
  (Utilities|Time|SetTimerbyEvent (delegate Custom|Wink%20Out) (Variables|Default|GetLifetime))
  ;[0.15 0.09377 0 0.5] Sphere Overlap
  (Collision|AssignOnComponentBeginOverlap (Variables|Default|GetSphere%20Volume) (delegate Custom|On%20Sphere%20Overlap)))

(event EventTick
  (params (DeltaSeconds :type Float%20%28single-precision%29))
  ;[0.15 0.1301 0 0.5] Update Location and Rotation
  (CallFunction|UpdateLocation DeltaSeconds)
  (CallFunction|UpdateRotation DeltaSeconds))

(fn ConstructionScript)

(fn InitializeDeltaRotation
  (Variables|Movement|SetDelta%20Rotation (* (Math|Random|RandomRotator false) (Variables|MovementSettings|GetRotation%20Scale%20Factor))))

(fn UpdateLocation
  (params (Delta%20Seconds :type Float%20%28double-precision%29))
  (Transformation|AddActorWorldOffset (* (Transformation|GetActorForwardVector) (* Delta%20Seconds (Variables|MovementSettings|GetSpeed)))))

(fn UpdateRotation
  (params (Delta%20Seconds :type Float%20%28double-precision%29))
  (Class|Actor|AddActorWorldRotation (* (Variables|Movement|GetDelta%20Rotation) (Utilities|Time|GetWorldDeltaSeconds))))

(fn UpdateScale
  (params (Scale :type Float%20%28double-precision%29))
  (Transformation|SetWorldScale3D (Variables|Default|GetSphere%20Mesh) (Math|Vector|MakeVector Scale Scale Scale)))