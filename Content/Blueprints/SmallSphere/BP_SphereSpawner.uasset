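; BP_SphereSpawner is an actor that periodically spawns BP_SmallSphere actors around itself.
; On BeginPlay it starts a looping timer at Interval, with the first spawn delayed by the same amount.
; Each tick of the timer places a sphere with random rotation at a random direction and distance up to MaxRange from the actor, adjusting for collision but always spawning.
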(event Custom|Spawn%20Sphere
  (bind _point (CallFunction|GetRandomPointinRange))
  (Game|SpawnActorfromClass "/Game/Blueprints/SmallSphere/BP_SmallSphere.BP_SmallSphere_C" (Math|Transform|MakeTransform _point (Math|Random|RandomRotator false) "1.000000,1.000000,1.000000") "AdjustIfPossibleButAlwaysSpawn" "MultiplyWithRoot" 0 0))

(event EventBeginPlay
  (bind _interval (Variables|SpawnSettings|GetInterval))
  (Utilities|Time|SetTimerbyEvent (delegate Custom|Spawn%20Sphere) _interval true true _interval))

(fn ConstructionScript)

(fn GetRandomPointinRange
  (return (+ (Transformation|GetActorLocation) (* (Math|Vector|GetForwardVector (Math|Random|RandomRotator false)) (Math|Random|RandomFloatinRange 0.0 (Variables|SpawnSettings|GetMax%20Range))))))