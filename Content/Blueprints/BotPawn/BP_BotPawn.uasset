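; Player-controlled bot pawn that flies with free 3D movement, adds the Enhanced Input mapping and overlay HUD, and fires beam projectiles.
; Movement follows control-rotation axes through FloatingPawnMovement, and Tick snaps actor rotation to control rotation.
; Firing alternates between rifle sockets, aiming each spawned BP_PlayerBeam at a camera sphere-trace hit or trace end, with burst VFX and sound.
; GetHit subtracts and prints Health, with no death handling.
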(event Input|EnhancedActionEvents|EnhancedInputActionAI_Fire
  (params (ActionValue :type Boolean) (ElapsedSeconds :type Float%20%28double-precision%29) (TriggeredSeconds :type Float%20%28double-precision%29) (InputAction :type Input%20Action%20Object%20Reference :default "/Game/Blueprints/Input/InputActions/AI_Fire.AI_Fire"))
  (bind _isa (Utilities|FlowControl|FlipFlop)
    (:A
      _)
    (:B
      _))
  (Combat|FireBeam _isa))

(event Input|EnhancedActionEvents|EnhancedInputActionAI_Look
  (params (ActionValue :type Vector%202D%20Structure) (ElapsedSeconds :type Float%20%28double-precision%29) (TriggeredSeconds :type Float%20%28double-precision%29) (InputAction :type Input%20Action%20Object%20Reference :default "/Game/Blueprints/Input/InputActions/AI_Look.AI_Look"))
  (bind (_x _y) (Math|Vector2D|BreakVector2D ActionValue))
  (Pawn|Input|AddControllerYawInput _x)
  (Pawn|Input|AddControllerPitchInput _y))

(event Input|EnhancedActionEvents|EnhancedInputActionAI_Move
  (params (ActionValue :type Vector :default "0, 0, 0") (ElapsedSeconds :type Float%20%28double-precision%29) (TriggeredSeconds :type Float%20%28double-precision%29) (InputAction :type Input%20Action%20Object%20Reference :default "/Game/Blueprints/Input/InputActions/AI_Move.AI_Move"))
  (Class|PawnMovementComponent|AddInputVector (Variables|Default|GetFloatingPawnMovement) (CallFunction|GetMovementVector ActionValue) false))

(event EventBeginPlay
  ;[0.15 0.03307 0.03307 0.5] Add Bot Input Mapping
  (bind _asplayer_controller (Utilities|Casting|CastToPlayerController (Pawn|GetController)))
  (Input|AddMappingContext (PlayerController|LocalPlayerSubsystems|GetEnhancedInputLocalPlayerSubsystem _asplayer_controller) "/Game/Blueprints/Input/IMC_Bot.IMC_Bot" 0 "(bIgnoreAllPressedKeysUntilRelease=True,bForceImmediately=False,bNotifyUserSettings=False)")
  (bind _returnvalue (UserInterface|CreateWidget "/Game/Blueprints/UI/WBP_OverlayHUD.WBP_OverlayHUD_C"))
  (UserInterface|Viewport|AddtoViewport _returnvalue 0))

(event EventGetHit
  (params (Damage :type Float%20%28double-precision%29) (Spawn%20Location :type Vector :default "0, 0, 0"))
  (bind _output_get (Variables|Combat|SetHealth (- (Variables|Combat|GetHealth) Damage)))
  (Development|PrintString (Utilities|String|ToString(Float) _output_get) true true "(R=1.000000,G=0.000000,B=0.000000,A=1.000000)" 2e+02 "HP"))

(event EventTick
  (params (DeltaSeconds :type Float%20%28single-precision%29))
  (Transformation|SetActorRotation (Pawn|GetControlRotation :!class /Script/Engine.Pawn)))

(fn ConstructionScript
  (Variables|Combat|SetHealth (Variables|CombatSettings|GetMax%20Health)))

(fn FireBeam
  (params (Is%20Right :type Boolean))
  (bind _aim_location (CallFunction|GetAimLocation))
  (LocalVariables|SetAim%20Location _aim_location)
  (if Is%20Right
    (Variables|Default|SetRifle%20Socket "Rifle_R")
    (else
      (Variables|Default|SetRifle%20Socket "Rifle_L")))
  (bind _returnvalue (Game|SpawnActorfromClass "/Game/Blueprints/Beam/BP_PlayerBeam.BP_PlayerBeam_C" (Math|Transform|MakeTransform (.location (Transformation|GetSocketTransform (Variables|Default|GetBot%20Mesh) (Variables|Default|GetRifle%20Socket) "RTS_World")) (Math|Rotator|FindLookatRotation (.location (Transformation|GetSocketTransform (Variables|Default|GetBot%20Mesh) (Variables|Default|GetRifle%20Socket) "RTS_World")) (LocalVariables|GetAim%20Location)) "1.000000,1.000000,1.000000") "AlwaysSpawn" "MultiplyWithRoot" self 0))
  (Default|SetProjectileSpeed _returnvalue (Variables|CombatSettings|GetProjectile%20Speed))
  (Default|SetProjectileDamage _returnvalue (Variables|CombatSettings|GetProjectile%20Damage))
  (Niagara|SpawnSystematLocation "/Game/Assets/Effects/NS_PlayerBurst.NS_PlayerBurst" (.location (Transformation|GetSocketTransform (Variables|Default|GetBot%20Mesh) (Variables|Default|GetRifle%20Socket) "RTS_World")) (.rotation (Transformation|GetSocketTransform (Variables|Default|GetBot%20Mesh) (Variables|Default|GetRifle%20Socket) "RTS_World")))
  (Audio|PlaySoundatLocation "/Game/Sound/Beam/MS_Beam.MS_Beam" (.location (Transformation|GetSocketTransform (Variables|Default|GetBot%20Mesh) (Variables|Default|GetRifle%20Socket) "RTS_World")) "0, 0, 0" 0.7 1.0 0.0 0 0 0 0))

(fn GetMovementVector
  (params (Movement%20Vector :type Vector))
  (bind (_x _y _z) (Math|Vector|BreakVector Movement%20Vector))
  (return (+ (* (Math|Vector|GetRightVector (Pawn|GetControlRotation :!class /Script/Engine.Pawn)) _x) (* (Math|Vector|GetForwardVector (Pawn|GetControlRotation :!class /Script/Engine.Pawn)) _y) (* (Math|Vector|GetUpVector (Pawn|GetControlRotation :!class /Script/Engine.Pawn)) _z))))

(fn GetStartEndVector
  (params (Trace%20Max%20Distance :type Float%20%28double-precision%29))
  (bind _returnvalue (Transformation|GetActorLocation))
  (return _returnvalue (+ _returnvalue (* (Transformation|GetActorForwardVector) Trace%20Max%20Distance))))

(fn GetComponentStartEndVector
  (params (Component :type Scene%20Component%20Object%20Reference) (Trace%20Max%20Distance :type Float%20%28double-precision%29))
  (bind _returnvalue (Transformation|GetWorldLocation Component))
  (return _returnvalue (+ _returnvalue (* (Math|Vector|GetForwardVector Component) Trace%20Max%20Distance))))

(fn GetAimLocation
  (bind _camera (Variables|Default|GetCamera))
  (bind _trace_max_distance (Variables|CombatSettings|GetTrace%20Max%20Distance))
  (bind (_start _end) (CallFunction|GetComponentStartEndVector _camera _trace_max_distance))
  (bind (_outhit _returnvalue) (Collision|SphereTraceByChannel _start _end 5e+01 "TraceTypeQuery1" false 0 "None"))
  (if _returnvalue
    (return (.Location (Collision|BreakHitResult _outhit)))
    (else
      (return _end))))